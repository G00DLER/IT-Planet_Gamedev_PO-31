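; Base inventory item actor that shows a floating name label while the main character overlaps it.
; The construction script builds the label from a Russian "Item:" prefix and the NameItem variable.
; Begin and end overlap toggle the label's visibility for BP_MainCharacter only.
; While the label is visible, Tick sets its yaw opposite to the player character's actor yaw, a simple billboard that ignores the camera.
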(event `self.ReceiveTick`
  (params (DeltaSeconds :type "Float (single-precision)"))
  (if (`SceneComponent.bVisible` (`self.Name`))
    (bind _asbp_main_character (cast `/Game/Blueprints/Characters/BP_MainCharacter` (`GameplayStatics.GetPlayerCharacter` 0)))
    (bind (_returnvalue_roll _returnvalue_pitch _returnvalue_yaw) (`KismetMathLibrary.BreakRotator` (`self.K2_GetActorRotation` _asbp_main_character)))
    (`SceneComponent.K2_SetWorldRotation` (`self.Name`) (`KismetMathLibrary.MakeRotator` 0.0 0.0 (+ _returnvalue_yaw 180.0)) false false)))

(event `self.ReceiveActorBeginOverlap`
  (params (OtherActor :type "Actor Object Reference"))
  (cast `/Game/Blueprints/Characters/BP_MainCharacter` OtherActor)
  (`SceneComponent.SetVisibility` (`self.Name`) true false))

(event `self.ReceiveActorEndOverlap`
  (params (OtherActor :type "Actor Object Reference"))
  (cast `/Game/Blueprints/Characters/BP_MainCharacter` OtherActor)
  (`SceneComponent.SetVisibility` (`self.Name`) false false))

(fn `UserConstructionScript`
  (`TextRenderComponent.K2_SetText` (`self.Name`) (`KismetTextLibrary.Conv_StringToText` (`KismetStringLibrary.Concat_StrStr` "Предмет: " (`self.Name_Item`)))))