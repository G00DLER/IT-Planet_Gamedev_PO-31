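; Player character Blueprint that handles movement, mouse look and switching between first- and third-person views.
; Axis inputs drive movement along actor forward and right vectors plus controller pitch and yaw, while Jump and Run inputs are delegated to StaminaComponent.
; ChangeViewPerson toggles on the camera's UsePawnControlRotation, swapping control rotation between Camera and SpringArm, resetting their relative transforms and setting per-view arm length and socket offset.
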(event `InputAxis|Move Forward / Backward`
  (params (AxisValue :type "Float (single-precision)"))
  ;[1 1 1] Управление
  ;;[1 1 1] Передвижение
  (`self.AddMovementInput` (`self.GetActorForwardVector`) AxisValue))

(event `InputAxis|Look Up / Down Mouse`
  (params (AxisValue :type "Float (single-precision)"))
  ;[1 1 1] Управление
  ;;[1 1 1] Мышка
  (`self.AddControllerPitchInput` AxisValue))

(event `InputAxis|Look Right / Left Mouse`
  (params (AxisValue :type "Float (single-precision)"))
  ;[1 1 1] Управление
  ;;[1 1 1] Мышка
  (`self.AddControllerYawInput` AxisValue))

(event `InputAxis|Move Right / Left`
  (params (AxisValue :type "Float (single-precision)"))
  ;[1 1 1] Управление
  ;;[1 1 1] Передвижение
  (`self.AddMovementInput` (`self.GetActorRightVector`) AxisValue))

(event `InputAction|ChangeView`
  (params (Key :type "Key Structure"))
  ;[1 1 1] Управление
  ;;[1 1 1] Смена вида лица
  (:`Pressed`
    (`self.Change_View_Person`)))

(event `InputAction|Jump`
  (params (Key :type "Key Structure"))
  ;[1 1 1] Управление
  ;;[1 1 1] Прыжок
  (:`Pressed`
    (`/Game/Blueprints/Components/BP_StaminaComponent.OnJumped` (`self.StaminaComponent`))))

(event `InputAction|Run`
  (params (Key :type "Key Structure"))
  (bind _staminacomponent (`self.StaminaComponent`))
  ;[1 1 1] Управление
  ;;[1 1 1] Бег
  (:`Pressed`
    (`/Game/Blueprints/Components/BP_StaminaComponent.Press Run` _staminacomponent))
  (:`Released`
    (`/Game/Blueprints/Components/BP_StaminaComponent.Released_Run` _staminacomponent)))

(fn `Change_View_Person`
  (bind _camera (`self.Camera`))
  (bind _springarm (`self.SpringArm`))
  (bind _camera_2 (`self.Camera`))
  (bind _springarm_2 (`self.SpringArm`))
  (if (`CameraComponent.bUsePawnControlRotation` (`self.Camera`))
    (set `CameraComponent.bUsePawnControlRotation` false _camera_2)
    (`SceneComponent.K2_SetRelativeLocationAndRotation` :`self` _camera_2)
    (set `SpringArmComponent.bUsePawnControlRotation` true _springarm_2)
    (`SceneComponent.K2_SetRelativeLocationAndRotation` :`self` _springarm_2)
    (set `SpringArmComponent.TargetArmLength` (`self.ThirdPersonLength`) _springarm_2)
    (set `SpringArmComponent.SocketOffset` (`self.ThirdPerson`) _springarm_2)
    (else
      (set `CameraComponent.bUsePawnControlRotation` true _camera)
      (`SceneComponent.K2_SetRelativeLocationAndRotation` :`self` _camera)
      (set `SpringArmComponent.bUsePawnControlRotation` false _springarm)
      (`SceneComponent.K2_SetRelativeLocationAndRotation` :`self` _springarm)
      (set `SpringArmComponent.TargetArmLength` (`self.FirstPersonLength`) _springarm)
      (set `SpringArmComponent.SocketOffset` (`self.FirstPerson`) _springarm))))

(fn `UserConstructionScript`
  (`parent.UserConstructionScript`))