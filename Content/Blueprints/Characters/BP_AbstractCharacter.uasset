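; BP_AbstractCharacter is a character Blueprint with health and inventory components, apparently meant as a base for player characters.
; On BeginPlay it binds to the HealthComponent's death and health-change dispatchers.
; Health changes print the new value to screen, and death prints a message and disables input.
; A separate DebugGraph holds unwired test snippets for applying damage, adding an inventory item and listing items.
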(event Custom|OnDead
  ;[1 1 1] Подписка на делегат смерти
  (Development|PrintString "You DEAD!" true true "(R=1.000000,G=0.000000,B=0.024231,A=1.000000)" 2e+01)
  (Input|DisableInput 0))

(event Custom|OnHealthChanged
  (params (NewHealth :type Float%20%28double-precision%29))
  ;[1 1 1] Подписка на делегат изменения здоровья
  (Development|PrintString (Utilities|String|Append "Здоровье игрока: " (Utilities|String|ToString(Float) NewHealth)) true true "(R=0.000000,G=0.660000,B=1.000000,A=1.000000)" 2e+01))

(event EventBeginPlay
  (Utilities|FlowControl|Sequence
    (:then_0
      ;[1 1 1] Подписка на делегат смерти
      (EventDispatchers|BindEventtoOnDeadDispatcher (Variables|Default|GetHealthComponent) (delegate Custom|OnDead)))
    (:then_1
      ;[1 1 1] Подписка на делегат изменения здоровья
      (EventDispatchers|BindEventtoOnHealthChangedDispatcher (Variables|Default|GetHealthComponent) (delegate Custom|OnHealthChanged)))))

(event Input|KeyboardEvents|DebugKeyF
  (params (Key :type Key%20Structure :default "None") (ActionValue :type Input%20Action%20Value%20Structure))
  ;[1 1 1] Дебаг для проверки нанесения урона
)

(event Input|KeyboardEvents|DebugKeyJ
  (params (Key :type Key%20Structure :default "None") (ActionValue :type Input%20Action%20Value%20Structure))
  ;[1 1 1] Дебаг для проверки добавления предмета
)

(event Input|KeyboardEvents|DebugKeyK
  (params (Key :type Key%20Structure :default "None") (ActionValue :type Input%20Action%20Value%20Structure))
  ;[1 1 1] Дебаг для проверки добавления предмета
)

(fn ConstructionScript)