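; Health component that tracks a character's health and announces changes and death through event dispatchers.
; On BeginPlay it caches its BP_AbstractCharacter owner and binds to that actor's AnyDamage event, routing damage into ChangeHealth.
; Damage is reduced by subtracting GetPercentArmor from the owner's ArmorComponent as a flat amount, with no clamping.
; Healing adds directly and broadcasts the change; zero or below broadcasts only death, and SetHealth assigns silently.
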(event `self.ReceiveBeginPlay`
  (bind _owner (`self.Owner`))
  (`|ExecutionSequence`
    (:`then_0`
      ;[1 1 1] Добавление переменной владельца компонента
      (bind _asbp_abstract_character (cast `/Game/Blueprints/Characters/BP_AbstractCharacter` (`self.GetOwner`)))
      (set `self.Owner` _asbp_abstract_character))
    (:`then_1`
      ;[1 1 1] Подписка на делегат получения урона
      (`/Engine/EditorBlueprintResources/StandardMacros.IsValid` _owner
        (:`Is Valid`
          (add `Actor.OnTakeAnyDamage` _owner (delegate `OnTakeAnyDamage_Event`)))))))

(event `OnTakeAnyDamage_Event`
  (params (DamagedActor :type "Actor Object Reference") (Damage :type "Float (single-precision)") (DamageType :type "DamageType Object Reference") (InstigatedBy :type "Controller Object Reference") (DamageCauser :type "Actor Object Reference"))
  ;[1 1 1] Подписка на делегат получения урона
  (`self.ChangeHealth` Damage))

(fn `ChangeHealth`
  (params (Number :type "Float (double-precision)") (`Plus?` :type Boolean))
  (if `Plus?`
    (bind _output_get (set `self.Health` (+ Number (`self.Health`))))
    (`self.OnHealthChangedDispatcher` _output_get)
    (else
      (bind _armor (`/Game/Blueprints/Components/BP_ArmorComponent.Get_Percent_Armor` (`/Game/Blueprints/Characters/BP_AbstractCharacter.ArmorComponent` (`self.Owner`))))
      (bind _output_get_2 (set `self.Health` (- (`self.Health`) (- Number _armor))))
      (if (<= _output_get_2 0.0)
        (`self.OnDeadDispatcher`)
        (else
          (`self.OnHealthChangedDispatcher` (`self.Health`)))))))

(fn `SetHealth`
  (params (NewHealth :type "Float (double-precision)"))
  (set `self.Health` NewHealth))