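; Stamina component for BP_AbstractCharacter that gates running and jumping on remaining stamina.
; PressRun uses a self-calling looping timer to drain stamina at raised walk speed until release, standstill or low stamina triggers ReleasedRun.
; ReleasedRun restores base speed and starts UpStamina, a timer-driven regeneration blocked while interacting or airborne.
; OnJumped spends stamina to jump, the landed delegate resumes regeneration, and stamina changes print to screen.
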(event `self.ReceiveBeginPlay`
  ;[1 1 1] Получение владельца компонента
  (bind _asbp_abstract_character (cast `/Game/Blueprints/Characters/BP_AbstractCharacter` (`self.GetOwner`)))
  (bind _output_get (set `self.Owner` _asbp_abstract_character))
  (set `self.Character Movement` (`Character.CharacterMovement` _output_get)))

(event `Up Stamina`
  ;[1 1 1] Повышение стамины
  (bind _returnvalue (`KismetSystemLibrary.K2_SetTimerDelegate` (delegate `Up Stamina`) 0.1 true))
  (set `self.Released_Timer_Handle` _returnvalue)
  (if (`self.Is_Interact`)
    (`KismetSystemLibrary.K2_ClearAndInvalidateTimerHandle` (`self.Released_Timer_Handle`) :!label _label)
    (elif (`self.Is_Landed?`)
      (if (< (`self.Stamina_Amount`) (`self.Max_Stamina_Amount`))
        (set `self.Stamina_Amount` (+ (`self.Stamina_Amount`) (`self.Step_Plus_Stamina`)))
        (`KismetSystemLibrary.PrintString` (`KismetStringLibrary.Concat_StrStr` "Стамина: " (`KismetStringLibrary.Conv_DoubleToString` (`self.Stamina_Amount`))))
        (else
          (`KismetSystemLibrary.K2_ClearAndInvalidateTimerHandle` (`self.Released_Timer_Handle`))))
      (else
        (goto _label)))))

(event `Press Run`
  ;[1 1 1] Бег
  (set `self.Is_Interact` true)
  (bind _returnvalue (`KismetSystemLibrary.K2_SetTimerDelegate` (delegate `Press Run`) 0.3 true))
  (set `self.Press_Timer_Handle` _returnvalue)
  (if (`KismetMathLibrary.EqualExactly_VectorVector` (`MovementComponent.Velocity` (`self.Character Movement`)))
    (`self.Released Run` :!label _label_2)
    (elif (> (`self.Stamina_Amount`) 10.0)
      (if (`self.Is_Interact`)
        (set `self.Stamina_Amount` (- (`self.Stamina_Amount`) (`self.Step_Minus_Stamina`)))
        (set `CharacterMovementComponent.MaxWalkSpeed` (`self.Max_Speed`) (`self.Character Movement`))
        (`KismetSystemLibrary.PrintString` (`KismetStringLibrary.Concat_StrStr` "Стамина: " (`KismetStringLibrary.Conv_DoubleToString` (`self.Stamina_Amount`))))
        (else
          (goto _label_2)))
      (else
        (goto _label_2)))))

(event `Released Run`
  ;[1 1 1] Бег
  (`KismetSystemLibrary.K2_ClearAndInvalidateTimerHandle` (`self.Press_Timer_Handle`))
  (set `self.Is_Interact` false)
  (`self.Up Stamina`)
  (set `CharacterMovementComponent.MaxWalkSpeed` (`self.Base_Speed`) (`Character.CharacterMovement` (`self.Owner`))))

(event `On Jumped`
  ;[1 1 1] Прыжок
  (add `Character.LandedDelegate` (`self.Owner`) (delegate `On Landed`))
  (if (`self.Is_Landed?`)
    (if (> (`self.Stamina_Amount`) 10.0)
      (set `self.Stamina_Amount` (- (`self.Stamina_Amount`) (`self.Step_Minus_Jump`)))
      (set `self.Is_Interact` true)
      (`Character.Jump` (`self.Owner`))
      (set `self.Is_Landed?` false)
      (`KismetSystemLibrary.PrintString` (`KismetStringLibrary.Concat_StrStr` "Стамина: " (`KismetStringLibrary.Conv_DoubleToString` (`self.Stamina_Amount`))))
      (else
        (set `self.Is_Interact` false :!label _label_3)
        (`self.Up Stamina`)))
    (else
      (goto _label_3))))

(event `On Landed`
  (params (Hit :type "HitResult Structure (by ref)"))
  ;[1 1 1] Прыжок
  (set `self.Is_Landed?` true)
  (goto _label_3))