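; Armor component that tracks the equipped armor item for four slots: body, hands, hip and leg.
; ChangeArmor casts the incoming item to BP_AbstractArmorItem, stores it by its armor type, recalculates the total and calls the armor-changed dispatcher.
; RefreshAllArmor sums the Armor value of each valid slot into AllArmor.
; GetPercentArmor returns AllArmor divided by Amount, or prints a message when there is no armor.
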(event `self.ReceiveBeginPlay`)

(fn `Change_Armor`
  (params (ArmorItem :type "Actor Object Reference"))
  (bind _asbp_abstract_armor_item (cast `/Game/Blueprints/Items/Armor/BP_AbstractArmorItem` ArmorItem))
  (switch `/Game/Blueprints/Enums/E_TypeArmor` (`/Game/Blueprints/Items/Armor/BP_AbstractArmorItem.Type_Armor` _asbp_abstract_armor_item)
    (:`NewEnumerator0`
      (set `self.Body` _asbp_abstract_armor_item))
    (:`NewEnumerator1`
      (set `self.Hands` _asbp_abstract_armor_item))
    (:`NewEnumerator2`
      (set `self.Hip` _asbp_abstract_armor_item))
    (:`NewEnumerator3`
      (set `self.Leg` _asbp_abstract_armor_item)))
  (`self.Refresh_All_Armor`)
  (`self.OnArmorChangedDispatcher`))

(fn `Get_Percent_Armor`
  (returns (Armor :type "Float (double-precision)"))
  (locals (Amount :type "Float (double-precision)" :default 1.5))
  (if (> (`self.All_Armor`) 0.0)
    (return (/ (`self.All_Armor`) (`local.Amount`)))
    (else
      (`KismetSystemLibrary.PrintString` "Not Armor" true true (struct :`G` 0.66 :`B` 1.0 :`A` 1.0) 20.0))))

(fn `Refresh_All_Armor`
  (locals (Current :type "Float (double-precision)"))
  (bind _body (`self.Body`))
  (bind _leg (`self.Leg`))
  (bind _hands (`self.Hands`))
  (bind _hip (`self.Hip`))
  (`|ExecutionSequence`
    (:`then_0`
      (`/Engine/EditorBlueprintResources/StandardMacros.IsValid` _body
        (:`Is Valid`
          (set `local.Current` (+ (`/Game/Blueprints/Items/Armor/BP_AbstractArmorItem.Armor` _body) (`local.Current`))))))
    (:`then_1`
      (`/Engine/EditorBlueprintResources/StandardMacros.IsValid` _hands
        (:`Is Valid`
          (set `local.Current` (+ (`/Game/Blueprints/Items/Armor/BP_AbstractArmorItem.Armor` _hands) (`local.Current`))))))
    (:`then_2`
      (`/Engine/EditorBlueprintResources/StandardMacros.IsValid` _hip
        (:`Is Valid`
          (set `local.Current` (+ (`/Game/Blueprints/Items/Armor/BP_AbstractArmorItem.Armor` _hip) (`local.Current`))))))
    (:`then_3`
      (`/Engine/EditorBlueprintResources/StandardMacros.IsValid` _leg
        (:`Is Valid`
          (set `local.Current` (+ (`/Game/Blueprints/Items/Armor/BP_AbstractArmorItem.Armor` _leg) (`local.Current`))))))
    (:`then_4`
      (set `self.All_Armor` (`local.Current`)))))