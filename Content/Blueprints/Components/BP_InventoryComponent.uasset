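; Inventory component that stores items in separate weapon, armor and eat item arrays.
; AddItem tries casting the new item to each abstract item class in turn, using an IsAdded flag to skip later checks once stored, then fires the OnItemAdded dispatcher.
; DebugShowAllItems prints every stored item's name, plus the armor type for armor pieces.
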(fn `Add_Item`
  (params (`New Item` :type "Actor Object Reference"))
  (locals (Item :type "Actor Object Reference") (`IsAdded?` :type Boolean))
  (bind _isadded_ (`local.IsAdded?`))
  (set `local.Item` `New Item`)
  (`|ExecutionSequence`
    (:`then_0`
      (if (not _isadded_)
        (bind _asbp_abstract_weapon_item (cast `/Game/Blueprints/Items/Weapon/BP_AbstractWeaponItem` (`local.Item`)))
        (`KismetArrayLibrary.Array_Add` (`self.Weapon_Items`) _asbp_abstract_weapon_item)
        (set `local.IsAdded?` true :!label _label)
        (`self.OnItemAddedDispatcher`)))
    (:`then_1`
      (if (not _isadded_)
        (bind _asbp_abstract_armor_item (cast `/Game/Blueprints/Items/Armor/BP_AbstractArmorItem` (`local.Item`)))
        (`KismetArrayLibrary.Array_Add` (`self.Armor_Items`) _asbp_abstract_armor_item)
        (goto _label)))
    (:`then_2`
      (if (not _isadded_)
        (bind _asbp_abstract_eat_item (cast `/Game/Blueprints/Items/Eat/BP_AbstractEatItem` (`local.Item`)))
        (`KismetArrayLibrary.Array_Add` (`self.Eat_Items`) _asbp_abstract_eat_item)
        (goto _label)))))

(fn `Debug_Show_All_Items`
  (`|ExecutionSequence`
    (:`then_0`
      (if (not (`KismetArrayLibrary.Array_IsEmpty` (`self.Weapon_Items`)))
        (for _array_element (`self.Weapon_Items`)
          (`KismetSystemLibrary.PrintString` (`/Game/Blueprints/Items/BP_AbstractInventoryItem.Name_Item` _array_element)))))
    (:`then_1`
      (if (not (`KismetArrayLibrary.Array_IsEmpty` (`self.Armor_Items`)))
        (for _array_element_2 (`self.Armor_Items`)
          (`KismetSystemLibrary.PrintString` (`/Game/Blueprints/Items/BP_AbstractInventoryItem.Name_Item` _array_element_2))
          (`KismetSystemLibrary.PrintString` (`|GetEnumeratorNameAsString` (`/Game/Blueprints/Items/Armor/BP_AbstractArmorItem.Type_Armor` _array_element_2))))))
    (:`then_2`
      (if (not (`KismetArrayLibrary.Array_IsEmpty` (`self.Eat_Items`)))
        (for _array_element_3 (`self.Eat_Items`)
          (`KismetSystemLibrary.PrintString` (`/Game/Blueprints/Items/BP_AbstractInventoryItem.Name_Item` _array_element_3)))))))